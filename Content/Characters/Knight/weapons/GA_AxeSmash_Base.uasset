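; Base gameplay ability for the Knight's axe smash, a telegraphed overhead swing.
; On activation it spawns a BP_AttackDecal at the owner's transform, with shape and timing taken from AttackDecalStruct.
; After the decal's duration it plays the swing directly on the skeletal mesh, then restores Animation Blueprint mode after a fixed delay and ends.
; The graph itself applies no damage and never calls CommitAbility.
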(event Ability|EventActivateAbility
  (bind _returnvalue (Ability|GetActorInfo))
  (bind _attackdecalstruct (Variables|Default|GetAttackDecalStruct))
  (bind _duration (Variables|/Script/ArmedCombat.AttackDecalAsset|GetDuration _attackdecalstruct))
  (bind _returnvalue_2 (Game|SpawnActorfromClass "/Game/Characters/Knight/Attacks/BP_AttackDecal.BP_AttackDecal_C" (Transformation|GetActorTransform (.owneractor _returnvalue)) "AlwaysSpawn" "MultiplyWithRoot" 0 0))
  (Default|SetMaterialParameters _returnvalue_2 (Variables|/Script/ArmedCombat.RadialAttackDecalAsset|GetAttackAngle _attackdecalstruct) (Variables|/Script/ArmedCombat.RadialAttackDecalAsset|GetDynamicRadius _attackdecalstruct) (Variables|/Script/ArmedCombat.RadialAttackDecalAsset|GetInnerRadius _attackdecalstruct) (Variables|/Script/ArmedCombat.RadialAttackDecalAsset|GetOuterRadius _attackdecalstruct))
  (Default|SetAttackParameters _returnvalue_2 _duration)
  (Utilities|FlowControl|Delay _duration)
  (Components|Animation|PlayAnimation (.skeletalmeshcomponent _returnvalue) "/Game/Characters/Knight/Imports/ArmedCombatKnight_Anim_Armature_OverHeadSwing.ArmedCombatKnight_Anim_Armature_OverHeadSwing" false)
  (Utilities|FlowControl|Delay 1.0)
  (Components|Animation|SetAnimationMode (.skeletalmeshcomponent _returnvalue) "AnimationBlueprint")
  (Ability|EndAbility))

(event Ability|EventOnEndAbility
  (params (bWasCancelled :type Boolean)))