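; Gameplay ability for the Knight's axe smash, a telegraphed overhead swing.
; On activation it spawns a BP_AttackDecal at the owner's transform, shapes it through material parameters and passes it the forecast duration.
; After that delay it plays the swing directly on the skeletal mesh rather than as a montage, waits a fixed second, restores Animation Blueprint mode and ends.
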(event Ability|EventActivateAbility
  (bind _returnvalue (Ability|GetActorInfo))
  (bind _forecastduration (Variables|Default|GetForecastDuration))
  (bind _returnvalue_2 (Game|SpawnActorfromClass "/Game/Characters/Knight/Attacks/BP_AttackDecal.BP_AttackDecal_C" (Transformation|GetActorTransform (.owneractor _returnvalue)) "AlwaysSpawn" "MultiplyWithRoot" 0 0))
  (Default|SetMaterialParameters _returnvalue_2 0.5 0.75 0.2 0.5)
  (Default|SetAttackParameters _returnvalue_2 _forecastduration)
  (Utilities|FlowControl|Delay _forecastduration)
  (Components|Animation|PlayAnimation (.skeletalmeshcomponent _returnvalue) "/Game/Characters/Knight/Imports/ArmedCombatKnight_Anim_Armature_OverHeadSwing.ArmedCombatKnight_Anim_Armature_OverHeadSwing" false)
  (Utilities|FlowControl|Delay 1.0)
  (Components|Animation|SetAnimationMode (.skeletalmeshcomponent _returnvalue) "AnimationBlueprint")
  (Ability|EndAbility))