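; AI knight character that spots the player and ragdolls on demand.
; Pawn sensing filters for the third-person player character, then sets blackboard flags for having seen the player and whether they are within combat range.
; StartRagdoll enables full mesh physics, disables capsule collision, and adds a small push force to the root bone.
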(event OnSeePawn(PawnSensing)
  (params (Pawn :type Pawn%20Object%20Reference))
  (bind _self self)
  (bind _asbp_third_person_character (Utilities|Casting|CastToBP_ThirdPersonCharacter Pawn))
  (AI|Components|Blackboard|SetValueasBool (AI|GetBlackboard (AI|GetAIController _self)) (Utilities|Name|MakeLiteralName "HasSeenPlayer") true)
  (AI|Components|Blackboard|SetValueasBool (AI|GetBlackboard (AI|GetAIController self)) (Utilities|Name|MakeLiteralName "InCombatRange") (<= (Transformation|GetDistanceTo _asbp_third_person_character _self) (Variables|Default|GetCombatRange))))

(event Custom|StartRagdoll
  (bind _mesh (Variables|Character|GetMesh))
  (bind _capsulecomponent (Variables|Default|GetCapsuleComponent))
  (Class|SkeletalMeshComponent|SetAllBodiesSimulatePhysics _mesh true)
  (Physics|SetSimulatePhysics _mesh true)
  (Class|PrimitiveComponent|WakeAllRigidBodies _mesh)
  (Collision|SetCollisionEnabled _capsulecomponent "NoCollision")
  (Collision|SetCollisionResponsetoAllChannels _capsulecomponent "ECR_Ignore")
  (Physics|AddForce _mesh "100.000000,100.000000,0.000000" "Root" false))

(fn ConstructionScript)